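; BP_Spline_Water is a positional water sound actor that follows the player along a spline.
; On BeginPlay it caches the BP_Character_Traveler player and starts a MoveAudio loop that repeats on a short Delay.
; Each pass moves the Water and Arrow components to the spline point closest to the player, raised slightly in Z, so the sound stays at the nearest part of the spline.
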(event Custom|MoveAudio
  (bind _spline (Variables|Default|GetSpline))
  (bind _char_ref (Variables|Default|GetChar%20REF))
  (bind _returnvalue (Transformation|GetActorLocation _char_ref))
  (bind _returnvalue_2 (Spline|FindLocationClosesttoWorldLocation _spline _returnvalue "World"))
  (Transformation|SetWorldLocation (Variables|Default|GetArrow) (Math|Vector|MakeVector (.x _returnvalue_2) (.y _returnvalue_2) (+ (.z _returnvalue_2) 5e+01)) false false)
  (Utilities|FlowControl|Delay 0.05)
  (CallFunction|MoveAudio))

(event EventBeginPlay
  (bind _asbp_character_traveler (Utilities|Casting|CastToBP_Character_Traveler (Game|GetPlayerCharacter 0)))
  (Variables|Default|SetChar%20REF _asbp_character_traveler)
  (CallFunction|MoveAudio))

(fn ConstructionScript)