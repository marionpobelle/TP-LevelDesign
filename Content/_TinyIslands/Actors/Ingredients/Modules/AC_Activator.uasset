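; Activator component that lets its owning actor switch a list of linked actors on and off through their AC_Listener components.
; On BeginPlay it registers itself with each listener as a connected activator.
; Activation requests go out on every call, while deactivation requests are sent only if it is currently activated.
; A debug event draws persistent lines from the owner to each linked actor; older BI_Listener interface calls remain unconnected.
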(event Custom|On%20Deactivation
  (if (Variables|Default|GetIsActivated)
    (Variables|Default|SetIsActivated false)
    (for _array_element (Variables|Default|GetActorsToActivate)
      (if (Utilities|IsValid (Actor|GetComponentbyClass _array_element "/Game/_TinyIslands/Actors/Ingredients/Modules/AC_Listener.AC_Listener_C"))
        (Default|RequestDeactivation (Actor|GetComponentbyClass _array_element "/Game/_TinyIslands/Actors/Ingredients/Modules/AC_Listener.AC_Listener_C"))))))

(event Custom|On%20Activation
  (if (Variables|Default|GetIsActivated)
    _
    (else
      (Variables|Default|SetIsActivated true)))
  (for _array_element (Variables|Default|GetActorsToActivate)
    (if (Utilities|IsValid (Actor|GetComponentbyClass _array_element "/Game/_TinyIslands/Actors/Ingredients/Modules/AC_Listener.AC_Listener_C"))
      (Default|RequestActivation (Actor|GetComponentbyClass _array_element "/Game/_TinyIslands/Actors/Ingredients/Modules/AC_Listener.AC_Listener_C")))))

(event Custom|Show%20Linked%20Actors
  (CallFunction|DrawDebugLines))

(event EventBeginPlay
  (for _array_element (Variables|Default|GetActorsToActivate)
    (if (Utilities|IsValid (Actor|GetComponentbyClass _array_element "/Game/_TinyIslands/Actors/Ingredients/Modules/AC_Listener.AC_Listener_C"))
      (Default|AddConnectedActivator (Actor|GetComponentbyClass _array_element "/Game/_TinyIslands/Actors/Ingredients/Modules/AC_Listener.AC_Listener_C")))))

(event EventTick
  (params (DeltaSeconds :type Float%20%28single-precision%29)))

(fn SetActorstoActivate
  (params (Actors :type Array%20of%20Actor%20Object%20References))
  (for _array_element Actors
    (Utilities|Array|Add (Variables|Default|GetActorsToActivate) _array_element)))

(fn DrawDebugLines
  (Rendering|Debug|FlushPersistentDebugLines)
  (for _array_element (Variables|Default|GetActorsToActivate)
    (Rendering|Debug|DrawDebugLine (+ (Transformation|GetActorLocation (Components|GetOwner)) "0.000000,0.000000,10.000000") (Transformation|GetActorLocation _array_element) "(R=0.000000,G=0.671875,B=0.039760,A=1.000000)" 99999.0 2.0)))